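; Player character for the pushable actor system that can grab, push and release objects.
; Interact press and release, plus the forward and right movement axes, are forwarded to the ACPushCharacter component alongside normal control-yaw-relative movement.
; Walking off a ledge exits the push state, and a CanJumpInternal override blocks jumping while the component is pushing.
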(event `InputAction|Interact`
  (params (Key :type "Key Structure"))
  (bind _ac_pushcharacter (`self.AC_PushCharacter`))
  ;[1 0.5 0.5] Grab / Release Push Actor
  (:`Pressed`
    (`/Game/PushableActorProject/Blueprints/BasicPush/AC_PushCharacter.InteractPressed` _ac_pushcharacter))
  (:`Released`
    (`/Game/PushableActorProject/Blueprints/BasicPush/AC_PushCharacter.InteractReleased` _ac_pushcharacter)))

(event `InputAxis|MoveForward` :overrideparent false
  (params (AxisValue :type "Float (single-precision)"))
  ;[0.6205 0.8834 1] Default Character Movement & Camera Input
  ;;[1 1 1] DEFAULT MOVEMENT
  (`self.AddMovementInput` (`KismetMathLibrary.GetForwardVector` (`KismetMathLibrary.MakeRotator` 0.0 0.0 (.yaw (`self.GetControlRotation`)))) AxisValue)
  (`/Game/PushableActorProject/Blueprints/BasicPush/AC_PushCharacter.PushForward` (`self.AC_PushCharacter`) AxisValue) ; Add forward movement to component
)

(event `InputAxis|MoveRight` :overrideparent false
  (params (AxisValue :type "Float (single-precision)"))
  ;[0.6205 0.8834 1] Default Character Movement & Camera Input
  ;;[1 1 1] DEFAULT MOVEMENT
  (`self.AddMovementInput` (`KismetMathLibrary.GetRightVector` (`KismetMathLibrary.MakeRotator` 0.0 0.0 (.yaw (`self.GetControlRotation`)))) AxisValue)
  (`/Game/PushableActorProject/Blueprints/BasicPush/AC_PushCharacter.PushRight` (`self.AC_PushCharacter`) AxisValue) ; Add right movement to component
)

(event `self.OnWalkingOffLedge`
  (params (PreviousFloorImpactNormal :type "Vector Structure (by ref)") (PreviousFloorContactNormal :type "Vector Structure (by ref)") (PreviousLocation :type "Vector Structure (by ref)") (TimeDelta :type "Float (single-precision)"))
  ;[1 0.5 0.5] Release Push Actor if falling off ledge
  (`parent.OnWalkingOffLedge` PreviousFloorImpactNormal PreviousFloorContactNormal PreviousLocation TimeDelta)
  (`/Game/PushableActorProject/Blueprints/BasicPush/AC_PushCharacter.ExitPushState` (`self.AC_PushCharacter`)) ; Release while falling send to component
)

(fn `CanJumpInternal`
  (returns (ReturnValue :type Boolean))
  ;[1 0.5 0.5] STOP JUMPING WHILE IN PUSH STATE  - Add other jump requirements here or remove if desire the ability to jump while pushing
  (bind _returnvalue (`parent.CanJumpInternal`))
  (return (and _returnvalue (not (`/Game/PushableActorProject/Blueprints/BasicPush/AC_PushCharacter.bPushing` (`self.AC_PushCharacter`))))))

(fn `UserConstructionScript`)